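; Save game object that stores and restores the player's quest log and per-quest objective progress.
; SaveQuestLog copies the active and completed quest lists, while SaveQuestDetails records each quest's stage and objective progress in a map keyed by quest ID.
; LoadQuests re-adds each active quest through the quest log component, applies its saved stage and progress, then restores both lists on the component.
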(fn `LoadQuests`
  (params (QuestLogComponent :type "/Game/HordeCore/Blueprints/Quests/QuestLogComponent Object Reference"))
  (for _array_element (`self.CurrentActiveQuests`)
    (bind _returnvalue (`/Game/HordeCore/Blueprints/Quests/QuestLogComponent.AddNewQuest` QuestLogComponent _array_element))
    (bind (_progress _currentstage) (break `/Game/HordeCore/Blueprints/Quests/ObjectiveProgressSaveData` (`BlueprintMapLibrary.Map_Find` (`self.QuestProgress`) _array_element)))
    (set `/Game/HordeCore/Blueprints/Quests/Quest_Base.CurrentStage` _currentstage _returnvalue)
    (set `/Game/HordeCore/Blueprints/Quests/Quest_Base.CurrentObjectiveProgress` _progress _returnvalue))
  (set `/Game/HordeCore/Blueprints/Quests/QuestLogComponent.currentActiveQuests` (`self.CurrentActiveQuests`) QuestLogComponent)
  (set `/Game/HordeCore/Blueprints/Quests/QuestLogComponent.completedQuests` (`self.CompletedQuests`) QuestLogComponent))

(fn `SaveQuestDetails`
  (params (QuestBase :type "/Game/HordeCore/Blueprints/Quests/Quest_Base Object Reference"))
  (`BlueprintMapLibrary.Map_Add` (`self.QuestProgress`) (`/Game/HordeCore/Blueprints/Quests/Quest_Base.Quest_ID` QuestBase) (make `/Game/HordeCore/Blueprints/Quests/ObjectiveProgressSaveData` (`/Game/HordeCore/Blueprints/Quests/Quest_Base.CurrentObjectiveProgress` QuestBase) (`/Game/HordeCore/Blueprints/Quests/Quest_Base.CurrentStage` QuestBase))))

(fn `SaveQuestLog`
  (params (QuestLog :type "/Game/HordeCore/Blueprints/Quests/QuestLogComponent Object Reference"))
  (set `self.CurrentActiveQuests` (`/Game/HordeCore/Blueprints/Quests/QuestLogComponent.currentActiveQuests` QuestLog))
  (set `self.CompletedQuests` (`/Game/HordeCore/Blueprints/Quests/QuestLogComponent.completedQuests` QuestLog)))