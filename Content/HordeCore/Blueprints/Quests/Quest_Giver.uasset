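; Quest giver component that offers a data-table quest to the player when its owner is interacted with.
; InteractWith asks the player's QuestLogComponent whether the quest is already active, printing a notice if so, and returns the owner's display name either way.
; Otherwise DisplayQuest looks up the QuesData row and opens a W_QuestGiverWidget with the quest details and row name as its ID.
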(fn `DisplayQuest`
  (bind (_quesdata_datatable _quesdata_rowname) (break `DataTableRowHandle` (`self.QuesData`)))
  (bind _returnvalue (`|GetDataTableRow` _quesdata_datatable _quesdata_rowname)
    (:`then`
      (bind _returnvalue_2 (`|CreateWidget` "/Game/HordeCore/Blueprints/Quests/UI/W_QuestGiverWidget.W_QuestGiverWidget_C" null _returnvalue _quesdata_rowname))
      (`UserWidget.AddToViewport` _returnvalue_2 0))))

(fn `InteractWith`
  (returns (ObjectiveID :type String))
  (bind (_quesdata_datatable _quesdata_rowname) (break `DataTableRowHandle` (`self.QuesData`)))
  (bind _returnvalue (`KismetSystemLibrary.GetDisplayName` (`self.GetOwner`)))
  (if (not (`/Game/HordeCore/Blueprints/Quests/QuestLogComponent.QueryActiveQuest` (`/Game/FirstPerson/Blueprints/BP_FirstPersonCharacter.QuestLogComponent` (`/Game/HordeCore/Blueprints/Quests/Qust_CommonFunctionLibrary.GetPlayer`)) _quesdata_rowname))
    (`self.DisplayQuest`)
    (return _returnvalue)
    (else
      (`KismetSystemLibrary.PrintString` "Already on Quest")
      (return _returnvalue))))