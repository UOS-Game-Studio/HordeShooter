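; Base quest actor that tracks one quest's current-stage objectives and flags the quest completed when all are met.
; On BeginPlay it loads the stage from D_QuestData, binds to the player's objective-ID event and seeds one objective type from inventory counts.
; Reported IDs adjust a progress map, broadcasting increases.
; Reaching an objective's quantity shows a notification widget and rechecks completion; stage advancement is absent here.
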(event `self.ReceiveBeginPlay`
  (`self.GetQuestDetails`)
  (add `/Game/FirstPerson/Blueprints/BP_FirstPersonCharacter.OnObjectiveIDCalled` (`/Game/HordeCore/Blueprints/Quests/Qust_CommonFunctionLibrary.GetPlayer`) (`|CreateDelegate` :!event `On Objective IDHeard`))
  (for _array_element (`.Objectives_23_67B8ABBE42BA7DC8F403ADB61048330F` (break `/Game/HordeCore/Blueprints/Quests/F_StageDetails` (`self.CurrentStageDetails`)))
    (bind (_name _description _objectivetype _objectiveid) (break `/Game/HordeCore/Blueprints/Quests/F_ObjectiveDetails` _array_element))
    (if (`|EnumEquality` _objectivetype "NewEnumerator3")
      (bind _value (`/Game/HordeCore/Blueprints/Quests/InventoryComponent.QueryInventory` (`/Game/FirstPerson/Blueprints/BP_FirstPersonCharacter.InventoryComponent` (`/Game/HordeCore/Blueprints/Quests/Qust_CommonFunctionLibrary.GetPlayer`)) (`KismetStringLibrary.Conv_StringToName` _objectiveid)))
      (`self.On Objective IDHeard` _objectiveid _value)))
  (bind _return (`self.IsObjectivesComplete`))
  (set `self.questCompleted` _return))

(fn `GetObjectiveDetailsByID`
  (params (ObjectiveID :type String))
  (returns (`Array Element` :type "/Game/HordeCore/Blueprints/Quests/F_ObjectiveDetails Structure"))
  (for _array_element (`.Objectives_23_67B8ABBE42BA7DC8F403ADB61048330F` (break `/Game/HordeCore/Blueprints/Quests/F_StageDetails` (`self.CurrentStageDetails`)))
    (if (`KismetStringLibrary.EqualEqual_StrStr` (`.ObjectiveID_11_B48324D84561BD015A7E7C98234AFE08` (break `/Game/HordeCore/Blueprints/Quests/F_ObjectiveDetails` _array_element)) ObjectiveID)
      (return _array_element))))

(fn `GetQuestDetails`
  ;[1 1 1] What is the Current Quest stage + Objective Progress
  (bind _returnvalue (`|GetDataTableRow` "/Game/HordeCore/Blueprints/Quests/D_QuestData.D_QuestData" (`self.Quest_ID`))
    (:`then`
      (bind _output_get (set `self.QuestDetails` _returnvalue))
      (bind _output_get_2 (set `self.CurrentStageDetails` (`|GetArrayItem` (`.Stages_13_1022D0C741F1BA4A1CE3D7802B1713FB` (break `/Game/HordeCore/Blueprints/Quests/F_Quest_Details` _output_get)) (`self.CurrentStage`))))
      ;[1 1 1] Populate ObjectiveProgress
      (`BlueprintMapLibrary.Map_Clear` (`self.CurrentObjectiveProgress`))
      (for _array_element (`.Objectives_23_67B8ABBE42BA7DC8F403ADB61048330F` (break `/Game/HordeCore/Blueprints/Quests/F_StageDetails` _output_get_2))
        (`BlueprintMapLibrary.Map_Add` (`self.CurrentObjectiveProgress`) (`.ObjectiveID_11_B48324D84561BD015A7E7C98234AFE08` (break `/Game/HordeCore/Blueprints/Quests/F_ObjectiveDetails` _array_element))) ; All ID  Set to 0
      ))))

(fn `IsObjectiveComplete`
  (params (ObjectiveID :type String))
  (bind (_name _description _objectivetype _objectiveid _quantity) (break `/Game/HordeCore/Blueprints/Quests/F_ObjectiveDetails` (`self.GetObjectiveDetailsByID` ObjectiveID)))
  ;[1 1 1] Set Objective CVomplete, Display Weidget
  (if (>= (`BlueprintMapLibrary.Map_Find` (`self.CurrentObjectiveProgress`) (`local.ObjectiveID`)) _quantity)
    (bind _returnvalue (`|CreateWidget` "/Game/HordeCore/Blueprints/Quests/UI/W_QuestNotification.W_QuestNotification_C" null _description))
    (`UserWidget.AddToViewport` _returnvalue 0)
    (bind _return (`self.IsObjectivesComplete`))
    (set `self.questCompleted` _return)))

(fn `IsObjectivesComplete`
  (returns (Return :type Boolean))
  (locals (Local_AllComplete :type Boolean :default true))
  (for _array_element (`.Objectives_23_67B8ABBE42BA7DC8F403ADB61048330F` (break `/Game/HordeCore/Blueprints/Quests/F_StageDetails` (`self.CurrentStageDetails`)))
    (bind (_name _description _objectivetype _objectiveid) (break `/Game/HordeCore/Blueprints/Quests/F_ObjectiveDetails` _array_element))
    (if (not (>= (`BlueprintMapLibrary.Map_Find` (`self.CurrentObjectiveProgress`) _objectiveid) (`.Quantity_14_5D59CB7740A6D796E0AE848FE1FF12FC` (break `/Game/HordeCore/Blueprints/Quests/F_ObjectiveDetails` (`self.GetObjectiveDetailsByID` _objectiveid)))))
      (bind _output_get (set `local.Local_AllComplete` false))
      (return _output_get)))
  (return (`local.Local_AllComplete`)))

(fn `On Objective IDHeard`
  (params (ObjectiveID :type String) (Value :type Integer :default 1))
  (bind (_value _returnvalue) (`BlueprintMapLibrary.Map_Find` (`self.CurrentObjectiveProgress`) (`local.ObjectiveID`)))
  (if (> (`KismetMathLibrary.SignOfInteger` Value) 0)
    (if _returnvalue
      (if (< _value (`.Quantity_14_5D59CB7740A6D796E0AE848FE1FF12FC` (break `/Game/HordeCore/Blueprints/Quests/F_ObjectiveDetails` (`self.GetObjectiveDetailsByID` (`local.ObjectiveID`)))))
        (`BlueprintMapLibrary.Map_Add` (`self.CurrentObjectiveProgress`) (`local.ObjectiveID`) (+ _value (`local.Value`))) ; Add new Ojective Id
        (`self.IsObjectiveComplete` (`local.ObjectiveID`))
        (`self.OnObjectiveHeard`)
        (return))
      (else
        (return)))
    (else
      (`BlueprintMapLibrary.Map_Add` (`self.CurrentObjectiveProgress`) (`local.ObjectiveID`) (+ (`BlueprintMapLibrary.Map_Find` (`self.CurrentObjectiveProgress`) (`local.ObjectiveID`)) (`local.Value`))) ; Add new Ojective Id
      (return))))

(fn `UserConstructionScript`)