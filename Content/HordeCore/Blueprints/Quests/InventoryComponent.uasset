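; Quest inventory component that stores item quantities by name in a map and reports changes to the player's objective system.
; AddToInventory adds to the stored count, while QueryInventory returns it.
; Both add and remove call CallOnObjectiveIDCalled on BP_FirstPersonCharacter, using the item name as objective ID.
; RemoveFromInventory deletes the whole entry before looking up its count, so the reported value comes from an already removed key.
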(fn `AddToInventory`
  (params (ItemName :type Name) (Quantity :type Integer))
  (bind _content (`self.Content`))
  (`KismetSystemLibrary.PrintString` "Added to Inventory")
  (`BlueprintMapLibrary.Map_Add` _content ItemName (+ Quantity (`BlueprintMapLibrary.Map_Find` _content ItemName)))
  (bind _asbp_first_person_character (cast `/Game/FirstPerson/Blueprints/BP_FirstPersonCharacter` (`GameplayStatics.GetPlayerCharacter` 0)))
  (`/Game/FirstPerson/Blueprints/BP_FirstPersonCharacter.OnObjectiveIDCalled` _asbp_first_person_character (`KismetStringLibrary.Conv_NameToString` (`local.ItemName`)) (`local.Quantity`)))

(fn `QueryInventory`
  (params (Key :type "Name (by ref)"))
  (returns (Value :type Integer))
  (return (`BlueprintMapLibrary.Map_Find` (`self.Content`) Key)))

(fn `RemoveFromInventory`
  (params (ItemName :type "Name (by ref)"))
  (bind _content (`self.Content`))
  (`BlueprintMapLibrary.Map_Remove` _content ItemName)
  (bind _asbp_first_person_character (cast `/Game/FirstPerson/Blueprints/BP_FirstPersonCharacter` (`GameplayStatics.GetPlayerCharacter` 0)))
  (`/Game/FirstPerson/Blueprints/BP_FirstPersonCharacter.OnObjectiveIDCalled` _asbp_first_person_character (`KismetStringLibrary.Conv_NameToString` ItemName) (- (`BlueprintMapLibrary.Map_Find` _content ItemName) 1)))