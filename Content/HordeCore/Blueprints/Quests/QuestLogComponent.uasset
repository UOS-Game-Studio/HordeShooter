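; Quest log component that tracks active and completed quests by ID and handles turn-ins.
; Adding a quest spawns a Quest_Base actor to hold its state and shows it on a single reused W_QuestTracker widget.
; Turning in adds the current stage's XP reward to the BP_HordeGameMode score, then completes the quest, updating the lists, flagging the actor and broadcasting completion.
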(event `self.ReceiveBeginPlay`
  (bind _asbp_first_person_character (cast `/Game/FirstPerson/Blueprints/BP_FirstPersonCharacter` (`GameplayStatics.GetPlayerCharacter` 0)))
  (set `self.As BP First Person Character` _asbp_first_person_character)
  (bind _asbp_horde_game_mode (cast `/Game/HordeCore/Blueprints/Game/BP_HordeGameMode` (`GameplayStatics.GetGameMode`)))
  (set `self.As BP Horde Game Mode` _asbp_horde_game_mode))

(fn `AddNewQuest`
  (params (QuestID :type Name))
  (returns (ReturnValue :type "/Game/HordeCore/Blueprints/Quests/Quest_Base Object Reference"))
  (locals (spawsTransform :type "Transform Structure"))
  (`KismetArrayLibrary.Array_AddUnique` (`self.currentActiveQuests`) QuestID)
  (bind _returnvalue (`|SpawnActorFromClass` "/Game/HordeCore/Blueprints/Quests/Quest_Base.Quest_Base_C" (`local.spawsTransform`) "Undefined" "MultiplyWithRoot" null QuestID null))
  (`KismetArrayLibrary.Array_Add` (`self.currentQuests`) _returnvalue)
  (`self.TrackQuest` _returnvalue)
  (return _returnvalue))

(fn `CompleteQuest`
  (params (QuestID :type "Name (by ref)"))
  (`KismetArrayLibrary.Array_AddUnique` (`self.completedQuests`) QuestID)
  (`KismetArrayLibrary.Array_RemoveItem` (`self.currentActiveQuests`) QuestID)
  (bind _array_element (`self.GetQuestActor` QuestID))
  (set `/Game/HordeCore/Blueprints/Quests/Quest_Base.isTurnedIn` true _array_element)
  (`self.QuestCompleted` _array_element)
  (return))

(fn `GetQuestActor`
  (params (QuestID :type Name))
  (returns (`Array Element` :type "/Game/HordeCore/Blueprints/Quests/Quest_Base Object Reference"))
  (for _array_element (`self.currentQuests`)
    (if (== (`/Game/HordeCore/Blueprints/Quests/Quest_Base.Quest_ID` _array_element) QuestID)
      (return _array_element))))

(fn `QueryActiveQuest`
  (params (QuestID :type Name))
  (returns (ReturnValue :type Boolean))
  (return (`KismetArrayLibrary.Array_Contains` (`self.currentActiveQuests`) QuestID)))

(fn `QueryCompletedQuest`
  (params (QuestID :type Name))
  (returns (ReturnValue :type Boolean) (isTurnedIn :type Boolean))
  (bind _returnvalue (`KismetArrayLibrary.Array_Contains` (`self.completedQuests`) QuestID))
  (bind _array_element (`self.GetQuestActor` QuestID))
  (`/Engine/EditorBlueprintResources/StandardMacros.IsValid` _array_element
    (:`Is Valid`
      (return _returnvalue (`/Game/HordeCore/Blueprints/Quests/Quest_Base.isTurnedIn` _array_element)))
    (:`Is Not Valid`
      (return _returnvalue true))))

(fn `TrackQuest`
  (params (QuestActorRef :type "/Game/HordeCore/Blueprints/Quests/Quest_Base Object Reference"))
  (bind _trackerhud (`self.TrackerHUD`)
    (:`then`
      (`/Game/HordeCore/Blueprints/Quests/UI/W_QuestTracker.UpdateData` _trackerhud QuestActorRef))
    (:`else`
      (bind _returnvalue (`|CreateWidget` "/Game/HordeCore/Blueprints/Quests/UI/W_QuestTracker.W_QuestTracker_C" null QuestActorRef))
      (bind _output_get (set `self.TrackerHUD` _returnvalue))
      (`UserWidget.AddToViewport` _output_get -1))))

(fn `TurnInQuest`
  (params (QuestID :type Name))
  (`|ExecutionSequence`
    (:`then_0`
      (bind _array_element (`self.GetQuestActor` QuestID))
      (`/Game/HordeCore/Blueprints/Game/BP_HordeGameMode.UpdateScore` (`self.As BP Horde Game Mode`) (`.XPReward_10_18C6B3584ECB85D7FCE0B4B990CC0046` (break `/Game/HordeCore/Blueprints/Quests/F_StageDetails` (`/Game/HordeCore/Blueprints/Quests/Quest_Base.CurrentStageDetails` _array_element)))))
    (:`then_1`
      (`self.CompleteQuest` QuestID))))