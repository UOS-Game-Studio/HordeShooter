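; Base pickup component for HordeCore pickups whose effect applies immediately.
; On BeginPlay it runs the parent logic, then calls Action and Destructor in sequence, so the effect fires once as soon as play begins for the component.
; Action, Destructor and SetUp only forward to their parent versions, and Tick is disabled.
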(event `self.ReceiveBeginPlay`
  (`parent.ReceiveBeginPlay`)
  (`self.Action`)
  (`self.Destructor`))

(fn `Action`
  (`parent.Action`))

(fn `Destructor`
  (`parent.Destructor`))

(fn `SetUp`
  (`parent.SetUp`))