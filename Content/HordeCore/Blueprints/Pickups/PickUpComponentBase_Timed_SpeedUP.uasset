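; Timed pickup component, derived from a parent pickup component, that temporarily speeds up the player character.
; SetUp reads player 0's speed through message calls, caches it as OldSpeed and applies it scaled by NewSpeedMultiplier.
; Destructor writes the cached speed back before running the parent cleanup, while Action only calls the parent.
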(fn `Action`
  (`parent.Action`))

(fn `Destructor`
  (message `/Game/HordeCore/Blueprints/Pickups/I_PlayerStatUpdater.SetSpeed` (`GameplayStatics.GetPlayerCharacter` 0) (`self.OldSpeed`))
  (`parent.Destructor`))

(fn `SetUp`
  (`parent.SetUp`)
  (bind _speed (message `/Game/HordeCore/Blueprints/Pickups/I_PlayerStatUpdater.GetSpeed` (`GameplayStatics.GetPlayerCharacter` 0)))
  (bind _output_get (set `self.OldSpeed` _speed))
  (message `/Game/HordeCore/Blueprints/Pickups/I_PlayerStatUpdater.SetSpeed` (`GameplayStatics.GetPlayerCharacter` 0) (* _output_get (`self.NewSpeedMultiplier`))))