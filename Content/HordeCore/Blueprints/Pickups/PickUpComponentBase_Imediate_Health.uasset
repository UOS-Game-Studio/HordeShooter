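; Immediate health pickup component that adds its Health amount to the player character's health.
; The Action override runs the parent logic, then reads and writes player 0's health through message calls.
; Health is applied only when the total stays at or below a hardcoded cap of 100, so a pickup that would overshoot adds nothing instead of clamping.
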(fn `Action`
  (bind _returnvalue (`GameplayStatics.GetPlayerCharacter` 0))
  (`parent.Action`)
  (bind _health (message `/Game/HordeCore/Blueprints/Pickups/I_PlayerStatUpdater.GetHealth` _returnvalue))
  (bind _returnvalue_2 (+ _health (`self.Health`)))
  (if (<= _returnvalue_2 100.0)
    (message `/Game/HordeCore/Blueprints/Pickups/I_PlayerStatUpdater.SetHealth` _returnvalue _returnvalue_2)))