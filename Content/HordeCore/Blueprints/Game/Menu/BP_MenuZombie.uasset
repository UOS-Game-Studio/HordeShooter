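; BP_MenuZombie is a zombie character that wanders on its own, apparently as menu scene dressing.
; On BeginPlay it picks a random skeletal mesh, then briefly disables CharacterMovement for a random delay so that animations across instances do not stay in sync.
; RandomRoam sends it via AIMoveTo to a random reachable point within SearchRadius and calls itself again only on success.
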(event `Random Roam`
  (`|AIMoveTo` self (`NavigationSystemV1.K2_GetRandomReachablePointInRadius` (`self.K2_GetActorLocation`) (`self.SearchRadius`) null null) null 50.0
    (:`OnSuccess`
      (`self.Random Roam`))))

(event `self.ReceiveTick`
  (params (DeltaSeconds :type "Float (single-precision)")))

(event `self.ReceiveBeginPlay`
  (bind _charactermovement (`self.CharacterMovement`))
  (`SkeletalMeshComponent.SetSkeletalMeshAsset` (`self.Mesh`) (`KismetArrayLibrary.Array_Random` (`self.Meshes`)))
  ;[1 1 1] delay movement component by random time so that animations stop syncing
  (`ActorComponent.SetActive` _charactermovement false false)
  (`KismetSystemLibrary.Delay` (`KismetMathLibrary.RandomFloatInRange` 0.0 0.6))
  (`ActorComponent.SetActive` _charactermovement true false)
  (`self.Random Roam`))

(fn `UserConstructionScript`)