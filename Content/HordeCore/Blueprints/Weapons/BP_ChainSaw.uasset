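; BP_ChainSaw is a short-range chainsaw weapon for the player, implemented in its Fire event.
; When the player can fire and ammo remains, it spends one ammo, adds to the HordeGameMode shot count and line-traces forward from the camera, with debug drawing enabled.
; Hits push physics-simulating components, apply point damage with a multiplier for the head bone, and spawn a blood effect on any surface struck.
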(event `self.Fire`
  (bind _returnvalue (`GameplayStatics.GetPlayerCameraManager` 0))
  (bind _damage (`self.Damage`))
  (bind _currentammo (`self.CurrentAmmo`))
  (bind _returnvalue_2 (`Actor.GetActorForwardVector` _returnvalue))
  (bind _returnvalue_3 (`Actor.K2_GetActorLocation` _returnvalue))
  (if (`/Game/FirstPerson/Blueprints/BP_FirstPersonCharacter.CanFire` (`self.PlayerRef`))
    (if (> _currentammo 0)
      (set `self.CurrentAmmo` (- _currentammo 1))
      (bind _asbp_horde_game_mode (cast `/Game/HordeCore/Blueprints/Game/BP_HordeGameMode` (`GameplayStatics.GetGameMode`)))
      (`/Game/HordeCore/Blueprints/Game/BP_HordeGameMode.AddToShotCount` _asbp_horde_game_mode)
      (bind (_outhit _returnvalue_4) (`KismetSystemLibrary.LineTraceSingle` :`Start` _returnvalue_3 :`End` (+ _returnvalue_3 (* _returnvalue_2 150.0)) :`TraceChannel` "TraceTypeQuery1" :`bTraceComplex` true :`DrawDebugType` "ForDuration" :`DrawTime` 1.0))
      (if _returnvalue_4
        (bind (_bblockinghit _binitialoverlap _time _distance _location _impactpoint _normal _impactnormal _physmat _hitactor _hitcomponent _hitbonename) (`GameplayStatics.BreakHitResult` _outhit))
        (if (`self.IsSimulatingPhysics` _hitcomponent _hitbonename)
          (`self.AddImpulse` _hitcomponent (* (+ _location (`KismetMathLibrary.Normal` (- _location _returnvalue_3))) 70.0) _hitbonename false))
        (if (== _hitbonename "head")
          (bind _returnvalue_5 (- _returnvalue_2 _location))
          (`GameplayStatics.ApplyPointDamage` _hitactor (* (`self.HeadshotMultiplier`) _damage) _returnvalue_5 _outhit)
          (else
            (`GameplayStatics.ApplyPointDamage` _hitactor _damage _returnvalue_5 _outhit)))
        (`GameplayStatics.SpawnEmitterAtLocation` "/Game/ThirdParty/Polygon_BattleRoyale/FX/PS_FX_Blood.PS_FX_Blood" _impactpoint)))))