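; Standard horde-mode zombie that spawns with a random mesh and reports hits, kills and point rewards to BP_HordeGameMode.
; BeginPlay sets up physical animation, enabling its tick late to avoid an engine crash, and randomly delays movement to desync animations.
; Point damage reduces health and sets movement speed on surviving hits.
; Death may spawn a random pickup, then ragdolls the body, fires the death call and destroys the actor after a delay.
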(event `self.ReceivePointDamage`
  (params (Damage :type "Float (single-precision)") (DamageType :type "DamageType Object Reference") (HitLocation :type "Vector Structure") (HitNormal :type "Vector Structure") (HitComponent :type "PrimitiveComponent Object Reference") (BoneName :type Name) (ShotFromDirection :type "Vector Structure") (InstigatedBy :type "Controller Object Reference") (DamageCauser :type "Actor Object Reference") (HitInfo :type "HitResult Structure (by ref)"))
  (set `self.CurrentHealth` (- (`self.CurrentHealth`) Damage))
  (bind _asbp_horde_game_mode (cast `/Game/HordeCore/Blueprints/Game/BP_HordeGameMode` (`GameplayStatics.GetGameMode`)))
  (`/Game/HordeCore/Blueprints/Game/BP_HordeGameMode.AddToHitCount` _asbp_horde_game_mode)
  (bind _isdead (`self.Is Dead`))
  (if _isdead
    (`/Engine/EditorBlueprintResources/StandardMacros.DoOnce` false
      (:`Completed`
        (`self.SpawnPickup`)
        (`self.Ragdoll mesh`)
        (`CharacterMovementComponent.DisableMovement` (`self.CharacterMovement`))
        (`PrimitiveComponent.SetCollisionEnabled` (`self.CapsuleComponent`) "NoCollision")
        (bind _asbp_horde_game_mode_2 (cast `/Game/HordeCore/Blueprints/Game/BP_HordeGameMode` (`GameplayStatics.GetGameMode`)))
        (`/Game/HordeCore/Blueprints/Game/BP_HordeGameMode.ZombieKilled` _asbp_horde_game_mode_2 (`self.PointsReward`))
        (`self.ZombieDeath`)
        (`KismetSystemLibrary.Delay` 5.0)
        (`self.K2_DestroyActor`)))
    (else
      (set `self.MovementSpeed` 2.5))))

(event `self.ReceiveBeginPlay`
  (bind _charactermovement (`self.CharacterMovement`))
  (`SkeletalMeshComponent.SetSkeletalMeshAsset` (`self.Mesh`) (`KismetArrayLibrary.Array_Random` (`self.Meshes`)))
  (`|ExecutionSequence`
    (:`then_0`
      (`PhysicalAnimationComponent.SetSkeletalMeshComponent` (`self.PhysicalAnimation`) (`self.Mesh`))
      (`PhysicalAnimationComponent.ApplyPhysicalAnimationSettingsBelow` (`self.PhysicalAnimation`) (`self.Bone Name`) (make `PhysicalAnimationData` false 500.0 100.0 500.0 100.0) true)
      (`SkeletalMeshComponent.SetAllBodiesBelowSimulatePhysics` (`self.Mesh`) (`self.Bone Name`) true true)
      (`PrimitiveComponent.SetSimulatePhysics` (`self.Mesh`) true)
      ;[1 1 1] delay movement component by random time so that animations stop syncing
      (`ActorComponent.SetActive` _charactermovement false false)
      (`KismetSystemLibrary.Delay` (`KismetMathLibrary.RandomFloatInRange` 0.0 4.0))
      (`ActorComponent.SetActive` _charactermovement true false))
    (:`then_1`
      (set `self.CurrentHealth` (`self.StartingHealth`)))
    (:`then_2`
      ;[1 1 1] spawning from BP with PA enables, crashes engine.
      (`KismetSystemLibrary.Delay` 0.2)
      (`ActorComponent.SetComponentTickEnabled` (`self.PhysicalAnimation`) true))))

(event `self.ReceiveTick`
  (params (DeltaSeconds :type "Float (single-precision)")))

(event `PATrigger`
  (`/Engine/EditorBlueprintResources/StandardMacros.FlipFlop`
    (:`A`
      (set `self.isPADisabled` true)
      (`/Engine/EditorBlueprintResources/StandardMacros.DoOnce` false :!via `Reset` :!label _label
        (:`Completed`
          (`KismetSystemLibrary.K2_SetTimer` null "PATrigger" 0.2))))
    (:`B`
      (set `self.isPADisabled` false)
      (goto _label :!via `Reset`))))

(event `DisablePhysicalAnimation`
  (`SkeletalMeshComponent.SetAllBodiesBelowPhysicsBlendWeight` (`self.Mesh`) (`self.Bone Name`) (`KismetMathLibrary.FInterpTo` 1.0 0.0 (`GameplayStatics.GetWorldDeltaSeconds`) 10.0) false true))

(fn `Is Dead`
  (returns (IsDead :type Boolean))
  (return (<= (`self.CurrentHealth`) 0.0)))

(fn `SpawnPickup`
  (returns (SpawnedPickup :type Boolean))
  (if (<= (`KismetMathLibrary.RandomInteger` 100) (`self.PickupSpawnChance`))
    (bind _returnvalue (`|SpawnActorFromClass` "/Game/HordeCore/Blueprints/Pickups/PickUpBase.PickUpBase_C" (`self.GetTransform`) "Undefined" "MultiplyWithRoot" null null))
    (set `/Game/HordeCore/Blueprints/Pickups/PickUpBase.PickUpStatsEffectComponent` (`KismetArrayLibrary.Array_Random` (`self.PickupTypes`)) _returnvalue)
    (`/Game/HordeCore/Blueprints/Pickups/PickUpBase.InitialiseFromSpawn` _returnvalue)
    (return true)
    (else
      (return false))))

(fn `UserConstructionScript`)