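; Standard zombie enemy that tracks health from damage and destroys itself at zero.
; On BeginPlay it sets up physical animation and simulates physics below a configurable bone for hit reactions.
; Projectile overlaps on the capsule set full physics blend weight and start a timer that toggles a disable flag.
; The interpolated blend-out is unfinished: the logic that would call it is disconnected.
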(event `self.ReceiveAnyDamage`
  (params (Damage :type "Float (single-precision)") (DamageType :type "DamageType Object Reference") (InstigatedBy :type "Controller Object Reference") (DamageCauser :type "Actor Object Reference"))
  (set `self.CurrentHealth` (- (`self.CurrentHealth`) Damage))
  (bind _isdead (`self.Is Dead`))
  (if _isdead
    (`self.K2_DestroyActor`)))

(event `self.ReceiveBeginPlay`
  (`|ExecutionSequence`
    (:`then_0`
      (`PhysicalAnimationComponent.SetSkeletalMeshComponent` (`self.PhysicalAnimation`) (`self.Mesh`))
      (`PhysicalAnimationComponent.ApplyPhysicalAnimationSettingsBelow` (`self.PhysicalAnimation`) (`self.Bone Name`) (make `PhysicalAnimationData` false 500.0 100.0 500.0 100.0) true)
      (`SkeletalMeshComponent.SetAllBodiesBelowSimulatePhysics` (`self.Mesh`) (`self.Bone Name`) true true)
      (`PrimitiveComponent.SetSimulatePhysics` (`self.Mesh`) true))
    (:`then_1`
      (set `self.CurrentHealth` (`self.StartingHealth`)))))

(event `self.ReceiveActorBeginOverlap`
  (params (OtherActor :type "Actor Object Reference")))

(event `self.CapsuleComponent.OnComponentBeginOverlap`
  (params (OverlappedComponent :type "PrimitiveComponent Object Reference") (OtherActor :type "Actor Object Reference") (OtherComp :type "PrimitiveComponent Object Reference") (OtherBodyIndex :type Integer) (bFromSweep :type Boolean) (SweepResult :type "HitResult Structure (by ref)"))
  (cast `/Game/FirstPerson/Blueprints/BP_FirstPersonProjectile` OtherActor)
  (`SkeletalMeshComponent.SetAllBodiesBelowPhysicsBlendWeight` (`self.Mesh`) (`self.Bone Name`) 1.0 false true)
  (`KismetSystemLibrary.K2_SetTimer` null "PATrigger" 0.2))

(event `self.ReceiveTick`
  (params (DeltaSeconds :type "Float (single-precision)")))

(event `PATrigger`
  (`/Engine/EditorBlueprintResources/StandardMacros.FlipFlop`
    (:`A`
      (set `self.isPADisabled` true)
      (`/Engine/EditorBlueprintResources/StandardMacros.DoOnce` false :!via `Reset` :!label _label
        (:`Completed`
          (`KismetSystemLibrary.K2_SetTimer` null "PATrigger" 0.2))))
    (:`B`
      (set `self.isPADisabled` false)
      (goto _label :!via `Reset`))))

(event `DisablePhysicalAnimation`
  (`SkeletalMeshComponent.SetAllBodiesBelowPhysicsBlendWeight` (`self.Mesh`) (`self.Bone Name`) (`KismetMathLibrary.FInterpTo` 1.0 0.0 (`GameplayStatics.GetWorldDeltaSeconds`) 10.0) false true))

(fn `Is Dead`
  (returns (IsDead :type Boolean))
  (return (<= (`self.CurrentHealth`) 0.0)))

(fn `UserConstructionScript`)