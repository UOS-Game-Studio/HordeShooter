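; BP_Director runs the zombie wave loop, tracking the current wave and score.
; After a short startup delay, it line-traces from every BP_ZombieSpawner to the player, keeping spawners whose trace is blocked.
; Each kept spawner spawns GetNumZombiesToSpawn standard zombies with a behavior tree, binding their death events and counting successful spawns.
; Deaths decrement that count; at zero, the wave advances and spawning repeats.
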(event `self.ReceiveBeginPlay`
  (bind _outactors (`GameplayStatics.GetAllActorsOfClass` "/Game/HordeCore/Blueprints/Spawners/BP_ZombieSpawner.BP_ZombieSpawner_C"))
  (set `self.ZombieSpawnerList` _outactors)
  (`/Engine/EditorBlueprintResources/StandardMacros.DoOnce` false
    (:`Completed`
      (`KismetSystemLibrary.Delay` 5.0)
      (`self.SpawnZombies`))))

(fn `AddToScore`
  (params (SocreToAdd :type Integer))
  (set `self.IScore` (+ (`self.IScore`) SocreToAdd)))

(fn `GetCurrentWave`
  (returns (Wave :type Integer))
  (return (`self.ICurrentWave`)))

(fn `GetScore`
  (returns (Score :type Integer))
  (return (`self.IScore`)))

(fn `OnZombieDeath`
  (bind _result (`/Engine/EditorBlueprintResources/StandardMacros.DecrementInt` (`self.INumZombiesToKillThisWave`))
    (:`  `
      (if (<= _result 0)
        (`/Engine/EditorBlueprintResources/StandardMacros.IncrementInt` (`self.ICurrentWave`)
          (:`  `
            (`self.SpawnZombies`)))))))

(fn `SpawnZombies`
  (locals (SpawnersNotVisibleToPlayer :type "Array of /Game/HordeCore/Blueprints/Spawners/BP_ZombieSpawner Object Reference"))
  (`KismetArrayLibrary.Array_Clear` (`local.SpawnersNotVisibleToPlayer`))
  (for _array_element (`self.ZombieSpawnerList`)
    (bind (_outhit _returnvalue) (`KismetSystemLibrary.LineTraceSingle` (`self.K2_GetActorLocation` _array_element) (`self.K2_GetActorLocation` (`GameplayStatics.GetPlayerPawn` 0)) "TraceTypeQuery1"))
    ;[1 1 1] if true, the line trace has hit an object between the spawner and the player. IE no line of sight
    (if _returnvalue
      (`KismetArrayLibrary.Array_Add` (`local.SpawnersNotVisibleToPlayer`) _array_element)))
  ;[1 1 1] reset for each wave
  (set `self.INumZombiesToKillThisWave` 0)
  ;[1 1 1] for each spawner
  (for _array_element_2 (`local.SpawnersNotVisibleToPlayer`)
    ;[1 1 1] for (zombies / spawners) ceil
    (for _ (range (`self.GetNumZombiesToSpawn`))
      (bind _returnvalue_2 (`AIBlueprintHelperLibrary.SpawnAIFromClass` "/Game/HordeCore/Blueprints/Zombies/BP_StandardZombie.BP_StandardZombie_C" "/Game/HordeCore/Blueprints/Zombies/BT_StandardZombie.BT_StandardZombie" (`self.K2_GetActorLocation` _array_element_2) (struct) false null))
      ;[1 1 1] bind to each zombies ZombieDeath event
      (bind _asbp_standard_zombie (cast `/Game/HordeCore/Blueprints/Zombies/BP_StandardZombie` _returnvalue_2))
      (add `/Game/HordeCore/Blueprints/Zombies/BP_StandardZombie.ZombieDeath` _asbp_standard_zombie (`|CreateDelegate` :!event `OnZombieDeath`))
      ;[1 1 1] wanted to do this more  gracfully but since zombies can be invalid after spawn, this makes more sence.
      (`/Engine/EditorBlueprintResources/StandardMacros.IncrementInt` (`self.INumZombiesToKillThisWave`)))))

(fn `UserConstructionScript`)